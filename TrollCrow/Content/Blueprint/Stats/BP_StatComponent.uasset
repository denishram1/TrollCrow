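; Stat component that holds stamina and chaos values, with only the stamina logic functional.
; The stamina modifier adds an amount, truncates to a whole number, clamps between zero and the maximum, then broadcasts OnStaminaChanged with current and max values.
; The chaos modifier is an unfinished stub: its similar clamp calculation is unconnected, so calling it changes nothing.
; The event graph holds only disabled default events.
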(event EventBeginPlay)

(event EventTick
  (params (DeltaSeconds :type Float%20%28single-precision%29)))

(fn ModifyChaos(floatAmount)
  (params (float%20Amount :type Float%20%28double-precision%29)))

(fn ModifyStamina(floatAmount)
  (params (Amount :type Float%20%28double-precision%29))
  (bind _output_get (Variables|Default|SetCurrentStamina (Math|Conversions|ToFloat(Integer) (Math|Integer|Clamp(Integer) (Math|Float|Truncate (+ (Variables|Default|GetCurrentStamina) Amount)) 0 (Math|Float|Truncate (Variables|Default|GetMaxStamina))))))
  (Default|CallOnStaminaChanged _output_get (Variables|Default|GetMaxStamina)))